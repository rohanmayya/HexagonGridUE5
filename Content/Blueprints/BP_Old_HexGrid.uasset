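; BP_Old_HexGrid is an actor that spawns a hexagon-shaped map of BP_Hex tiles at BeginPlay.
; CreateHexMap walks axial coordinates within MapRadius, clamping each row's range with Max and Min to form the hexagon outline.
; It places tiles at a fixed height using hard-coded spacing plus XOffset and YOffset to shift rows, and labels each tile with its coordinate pair.
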(event `self.ReceiveBeginPlay`
  (`self.CreateHexMap`))

(fn `CreateHexMap`
  (locals (MapRadius :type Integer :default 3) (R1 :type Integer) (R2 :type Integer) (XOffset :type "Float (double-precision)" :default -42.5) (YOffset :type "Float (double-precision)" :default -25.0))
  (bind _mapradius (`local.MapRadius`))
  (bind _mapradius_2 (`local.MapRadius`))
  (bind _mapradius_3 (`local.MapRadius`))
  (for _index (range (* _mapradius -1) (+ _mapradius 1))
    ;[1 1 1] R1
    (set `local.R1` (`KismetMathLibrary.Max` (- (* _index -1) _mapradius_2) (* _mapradius_2 -1)))
    ;[1 1 1] R2
    (set `local.R2` (`KismetMathLibrary.Min` _mapradius_3 (+ (* _index -1) _mapradius_3)))
    (for _index_2 (range (`local.R1`) (+ (`local.R2`) 1))
      (bind _returnvalue (`|SpawnActorFromClass` "/Game/Blueprints/BP_Hex.BP_Hex_C" (`KismetMathLibrary.MakeTransform` (`KismetMathLibrary.MakeVector` (+ (`KismetMathLibrary.Conv_IntToDouble` (* _index_2 85)) (* (`local.XOffset`) (* _index -1))) (+ (`KismetMathLibrary.Conv_IntToDouble` (* _index 100)) (* _index (`local.YOffset`))) 10.0)) "Undefined" "OverrideRootScale" null null))
      (`TextRenderComponent.K2_SetText` (`/Game/Blueprints/BP_Hex.Text` _returnvalue) (`KismetTextLibrary.Conv_StringToText` (`KismetStringLibrary.Concat_StrStr` (`KismetStringLibrary.Conv_IntToString` _index_2) "," (`KismetStringLibrary.Conv_IntToString` _index)))))))

(fn `UserConstructionScript`)